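; Rappel mesh actor that moves its static mesh vertically on player key presses.
; BeginPlay enables input from the first player controller.
; Up and Down presses call RopePositionUpdated with a fixed positive or negative step, which offsets the mesh's world Z location without sweep.
; Movement happens once per press rather than continuously, as Tick is unused.
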(event `self.ReceiveBeginPlay`
  (`self.EnableInput` (`GameplayStatics.GetPlayerController` 0)))

(event `Key|Up`
  (params (Key :type "Key Structure"))
  (:`Pressed`
    (`self.RopePositionUpdated` 5.0)))

(event `Key|Down`
  (params (Key :type "Key Structure"))
  (:`Pressed`
    (`self.RopePositionUpdated` -5.0)))

(event `RopePositionUpdated`
  (params (RopePositionChange :type "Float (double-precision)"))
  (`SceneComponent.K2_SetWorldLocation` (`self.StaticMeshComponent`) (+ (`KismetMathLibrary.MakeVector` 0.0 0.0 RopePositionChange) (`SceneComponent.K2_GetComponentLocation` (`self.StaticMeshComponent`))) false false))

(fn `UserConstructionScript`)