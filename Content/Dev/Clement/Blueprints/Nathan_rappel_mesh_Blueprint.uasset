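; Rappel actor, apparently a dev prototype, that plays a looping rappel animation on a skeletal mesh and lets the player move it along the rope.
; Up and Down key presses shift the mesh a fixed step in world Z through RopePositionUpdated.
; Tick adds a cosine-of-game-time swing along a rotated forward vector, scaled by BalanceAmplitude and applied per frame without delta time, making it frame-rate dependent.
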(event `self.ReceiveBeginPlay`
  (`self.EnableInput` (`GameplayStatics.GetPlayerController` 0))
  (`SkeletalMeshComponent.PlayAnimation` (`self.SkeletalMeshComponent`) "/Game/Dev/Clement/Animations/RappelAnim.RappelAnim" true))

(event `Key|Up`
  (params (Key :type "Key Structure"))
  (:`Pressed`
    (`self.RopePositionUpdated` 5.0)))

(event `Key|Down`
  (params (Key :type "Key Structure"))
  (:`Pressed`
    (`self.RopePositionUpdated` -5.0)))

(event `RopePositionUpdated`
  (params (RopePositionChange :type "Float (double-precision)"))
  (`SceneComponent.K2_SetWorldLocation` (`self.SkeletalMeshComponent`) (+ (`KismetMathLibrary.MakeVector` 0.0 0.0 RopePositionChange) (`SceneComponent.K2_GetComponentLocation` (`self.SkeletalMeshComponent`))) false false))

(event `self.ReceiveTick`
  (params (DeltaSeconds :type "Float (single-precision)"))
  (`SceneComponent.K2_SetWorldLocation` (`self.SkeletalMeshComponent`) (+ (`SceneComponent.K2_GetComponentLocation` (`self.SkeletalMeshComponent`)) (* (`KismetMathLibrary.GetForwardVector` (`KismetMathLibrary.ComposeRotators` (`SceneComponent.K2_GetComponentRotation` (`self.SkeletalMeshComponent`)) (struct :`Yaw` 90.0))) (* (`self.BalanceAmplitude`) (`KismetMathLibrary.Cos` (`KismetSystemLibrary.GetGameTimeInSeconds`))))) false false))

(fn `UserConstructionScript`)